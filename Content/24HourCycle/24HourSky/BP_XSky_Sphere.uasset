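; Sky sphere actor that runs a 24-hour day-night cycle with sun, clouds, stars and moon.
; Construction creates a dynamic panning-cloud material and fills its parameters.
; Tick advances CurrentTime, then SetInterpolateParam lerps sky colors, star brightness and the directional light's pitch, color and intensity between Morning, Noon, Dusk and Night keys at TimeTable hours.
; UpdateSunDirection feeds the light back into the material, using below-horizon sun height to blend in stars.
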(event EventBeginPlay
  ;[1 1 1] Initialize Light Source Direction
  (Variables|TimeDebugSettings|SetCurrent%20Time (.X (Math|Vector4|BreakVector4 (Variables|TimeDebugSettings|GetTimeTable))))
  (Transformation|SetActorRotation (Variables|Default|GetDirectional%20light%20actor) (Variables|Default|GetLightStartRotator))
  (CallFunction|UpdateSunDirection))

(event EventTick
  (params (DeltaSeconds :type Float%20%28single-precision%29))
  (bind _cycle_speed (Variables|TimeDebugSettings|GetCycle%20Speed))
  ;[1 1 1] Update Light Source Direction
  (Transformation|AddActorLocalRotation (Variables|Default|GetDirectional%20light%20actor) (Math|Rotator|MakeRotator 0.0 (/ -3.6e+02 (/ 1.44e+03 (* DeltaSeconds _cycle_speed))) 0.0) false false)
  (CallFunction|UpdateSunDirection)
  (if (>= (+ (/ (* DeltaSeconds _cycle_speed) 6e+01) (Variables|TimeDebugSettings|GetCurrent%20Time)) 24.0)
    (Variables|TimeDebugSettings|SetCurrent%20Time 0.0)
    (else
      (Variables|TimeDebugSettings|SetCurrent%20Time (+ (/ (* DeltaSeconds _cycle_speed) 6e+01) (Variables|TimeDebugSettings|GetCurrent%20Time)))))
  (CallFunction|SetInterpolateParam))

(fn ConstructionScript
  (bind _returnvalue (Rendering|Material|CreateDynamicMaterialInstance (Variables|BPSkydome|GetSkySphereMesh) 0 "/Game/24HourCycle/24HourSky/M_XSky_Panning_Clouds2.M_XSky_Panning_Clouds2" "None" :!class /Script/Engine.PrimitiveComponent))
  (Variables|Default|SetSky%20material _returnvalue)
  (if (Variables|Default|GetRefresh%20material) ; Updating bool in details panel causes construction script to run again
    _
    (else
      _))
  (Variables|Default|SetRefresh%20material false)
  (CallFunction|RefreshMaterial))

(fn UpdateSunDirection
  (bind _sky_material (Variables|Default|GetSky%20material))
  (Rendering|Material|SetVectorParameterValue _sky_material "Light direction" (Math|Conversions|ToLinearColor(Vector) (Math|Rotator|GetRotationXVector (Transformation|GetActorRotation (Variables|Default|GetDirectional%20light%20actor)))) :!class /Script/Engine.MaterialInstanceDynamic)
  (Rendering|Material|SetVectorParameterValue _sky_material "Sun color" (Math|Conversions|ToLinearColor(Color) (Variables|/Script/Engine.LightComponentBase|GetLightColor (Variables|/Script/Engine.Light|GetLightComponent (Variables|Default|GetDirectional%20light%20actor)))) :!class /Script/Engine.MaterialInstanceDynamic)
  (Variables|SunSettings|SetSun%20Height (Math|Float|MapRangeUnclamped (.Pitch (Math|Rotator|BreakRotator (Transformation|GetActorRotation (Variables|Default|GetDirectional%20light%20actor)))) 0.0 -9e+01 0.0 1.0))
  (Rendering|Material|SetScalarParameterValue (Variables|Default|GetSky%20material) "Sun height" (Math|Float|SelectFloat (Math|Float|Absolute(Float) (Variables|SunSettings|GetSun%20Height)) 0.0 (< (Variables|SunSettings|GetSun%20Height) 0.0)) :!class /Script/Engine.MaterialInstanceDynamic))

(fn RefreshMaterial
  (bind _sky_material (Variables|Default|GetSky%20material))
  (bind _sky_material_2 (Variables|Default|GetSky%20material))
  (bind _sky_material_3 (Variables|Default|GetSky%20material))
  (bind _sky_material_4 (Variables|Default|GetSky%20material))
  (bind _sky_material_5 (Variables|Default|GetSky%20material))
  (Utilities|IsValid (Variables|Default|GetDirectional%20light%20actor) ; Has a directional light been assigned?
    (:Is%20Valid
      (Rendering|Material|SetVectorParameterValue _sky_material_3 "Light direction" (Math|Conversions|ToLinearColor(Vector) (Math|Rotator|GetRotationXVector (Transformation|GetActorRotation (Variables|Default|GetDirectional%20light%20actor)))) :!class /Script/Engine.MaterialInstanceDynamic)
      (Rendering|Material|SetVectorParameterValue _sky_material_3 "Sun color" (Math|Conversions|ToLinearColor(Color) (Variables|/Script/Engine.LightComponentBase|GetLightColor (Variables|/Script/Engine.Light|GetLightComponent (Variables|Default|GetDirectional%20light%20actor)))) :!class /Script/Engine.MaterialInstanceDynamic)
      (Variables|SunSettings|SetSun%20Height (Math|Float|MapRangeUnclamped (.Pitch (Math|Rotator|BreakRotator (Transformation|GetActorRotation (Variables|Default|GetDirectional%20light%20actor)))) 0.0 -9e+01 0.0 1.0)))
    (:Is%20Not%20Valid
      (Rendering|Material|SetVectorParameterValue _sky_material_2 "Light direction" (Math|Conversions|ToLinearColor(Vector) (Math|Rotator|GetRotationXVector (Math|Rotator|MakeRotator 0.0 (Math|Float|MapRangeUnclamped (Variables|SunSettings|GetSun%20Height) -1.0 1.0 9e+01 -9e+01) (.Yaw (Math|Rotator|BreakRotator (Transformation|GetActorRotation)))))) :!class /Script/Engine.MaterialInstanceDynamic)
      (Rendering|Material|SetVectorParameterValue _sky_material_2 "Sun color" (Math|Color|Lerp(LinearColor) "(R=1.000000,G=0.221000,B=0.040000,A=1.000000)" "(R=0.954000,G=0.901000,B=0.744120,A=1.000000)" (Math|Float|Clamp(Float) (+ (Variables|SunSettings|GetSun%20Height) 0.2))) :!class /Script/Engine.MaterialInstanceDynamic)))
  (if (Variables|Default|GetColors%20determined%20by%20sun%20position)
    (Rendering|Material|SetVectorParameterValue _sky_material_5 "Horizon color" (Class|CurveLinearColor|GetClampedLinearColorValue (Variables|SkySettings|GetHorizon%20Color%20Curve) (Variables|SunSettings|GetSun%20Height)) :!class /Script/Engine.MaterialInstanceDynamic)
    (Rendering|Material|SetVectorParameterValue _sky_material_5 "Zenith color" (Class|CurveLinearColor|GetClampedLinearColorValue (Variables|SkySettings|GetZenith%20Color%20Curve) (Variables|SunSettings|GetSun%20Height)) :!class /Script/Engine.MaterialInstanceDynamic)
    (Rendering|Material|SetVectorParameterValue _sky_material_5 "CloudBrightColor" (Class|CurveLinearColor|GetClampedLinearColorValue (Variables|CloudSettings|GetCloud%20Color%20Curve) (Variables|SunSettings|GetSun%20Height)) :!class /Script/Engine.MaterialInstanceDynamic)
    (Rendering|Material|SetScalarParameterValue _sky_material_5 "Horizon falloff" (Math|Float|Lerp 3.0 7.0 (Math|Float|Absolute(Float) (Variables|SunSettings|GetSun%20Height))) :!class /Script/Engine.MaterialInstanceDynamic)
    (else
      (Rendering|Material|SetVectorParameterValue _sky_material "Horizon color" (Variables|SkySettings|GetHorizon%20Color) :!class /Script/Engine.MaterialInstanceDynamic)
      (Rendering|Material|SetVectorParameterValue _sky_material "Zenith color" (Variables|SkySettings|GetZenith%20Color) :!class /Script/Engine.MaterialInstanceDynamic)
      (Rendering|Material|SetVectorParameterValue _sky_material "CloudBrightColor" (Variables|CloudSettings|GetCloud%20Bright%20Color) :!class /Script/Engine.MaterialInstanceDynamic)
      (Rendering|Material|SetScalarParameterValue _sky_material "Horizon falloff" (Variables|SkySettings|GetHorizon%20Falloff) :!class /Script/Engine.MaterialInstanceDynamic)))
  (Rendering|Material|SetScalarParameterValue _sky_material_4 "SunSize" (Variables|SunSettings|GetSun%20Size) :!class /Script/Engine.MaterialInstanceDynamic)
  (Rendering|Material|SetScalarParameterValue _sky_material_4 "Sun height" (Math|Float|SelectFloat (Math|Float|Absolute(Float) (Variables|SunSettings|GetSun%20Height)) 0.0 (< (Variables|SunSettings|GetSun%20Height) 0.0)) :!class /Script/Engine.MaterialInstanceDynamic)
  (Rendering|Material|SetScalarParameterValue _sky_material_4 "SunSizeConvergence" (Variables|SunSettings|GetSun%20Size%20Convergence) :!class /Script/Engine.MaterialInstanceDynamic)
  (Rendering|Material|SetScalarParameterValue _sky_material_4 "Stars brightness" (Variables|StarSettings|GetStars%20Brightness) :!class /Script/Engine.MaterialInstanceDynamic)
  (Rendering|Material|SetScalarParameterValue _sky_material_4 "CloudAltitude" (Variables|CloudSettings|GetCloud%20Altitude) :!class /Script/Engine.MaterialInstanceDynamic)
  (Rendering|Material|SetScalarParameterValue _sky_material_4 "CloudSpeedX" (Variables|CloudSettings|GetCloud%20SpeedX) :!class /Script/Engine.MaterialInstanceDynamic)
  (Rendering|Material|SetScalarParameterValue _sky_material_4 "CloudSpeedY" (Variables|CloudSettings|GetCloud%20SpeedY) :!class /Script/Engine.MaterialInstanceDynamic)
  (Rendering|Material|SetScalarParameterValue _sky_material_4 "CloudAlphaThreshold" (Variables|CloudSettings|GetCloud%20Alpha%20Threshold) :!class /Script/Engine.MaterialInstanceDynamic)
  (Rendering|Material|SetScalarParameterValue _sky_material_4 "CloudAlphaIntensity" (Variables|CloudSettings|GetCloud%20Alpha%20Intensity) :!class /Script/Engine.MaterialInstanceDynamic)
  (Rendering|Material|SetScalarParameterValue _sky_material_4 "CloudDetailIntensity" (Variables|CloudSettings|GetCloud%20Detail%20Intensity) :!class /Script/Engine.MaterialInstanceDynamic)
  (Rendering|Material|SetScalarParameterValue _sky_material_4 "CloudBlendRange" (Variables|CloudSettings|GetCloud%20Blend%20Range) :!class /Script/Engine.MaterialInstanceDynamic)
  (Rendering|Material|SetScalarParameterValue _sky_material_4 "CloudBlendIntensity" (Variables|CloudSettings|GetCloud%20Blend%20Intensity) :!class /Script/Engine.MaterialInstanceDynamic)
  (Rendering|Material|SetVectorParameterValue _sky_material_4 "CloudDarkColor" (Variables|CloudSettings|GetCloud%20Dark%20Color) :!class /Script/Engine.MaterialInstanceDynamic)
  (Rendering|Material|SetScalarParameterValue _sky_material_4 "SunBrightness" (Variables|SunSettings|GetSun%20Brightness) :!class /Script/Engine.MaterialInstanceDynamic)
  (Rendering|Material|SetScalarParameterValue _sky_material_4 "BGStarDensity" (Variables|StarSettings|GetBGStarDensity) :!class /Script/Engine.MaterialInstanceDynamic)
  (Rendering|Material|SetScalarParameterValue _sky_material_4 "BGStarTwinkFrequence" (Variables|StarSettings|GetBGStarTwinkFrequence) :!class /Script/Engine.MaterialInstanceDynamic)
  (Rendering|Material|SetScalarParameterValue _sky_material_4 "TwinkFrequence" (Variables|StarSettings|GetTwinkFrequence) :!class /Script/Engine.MaterialInstanceDynamic)
  (Rendering|Material|SetScalarParameterValue _sky_material_4 "BigStarDensity" (Variables|StarSettings|GetBigStarDensity) :!class /Script/Engine.MaterialInstanceDynamic)
  (Rendering|Material|SetScalarParameterValue _sky_material_4 "BigStarDensity" (Variables|StarSettings|GetBigStarIntensity) :!class /Script/Engine.MaterialInstanceDynamic)
  (Rendering|Material|SetVectorParameterValue _sky_material_4 "NoiseColor01" (Variables|StarSettings|GetNoiseColor01) :!class /Script/Engine.MaterialInstanceDynamic)
  (Rendering|Material|SetVectorParameterValue _sky_material_4 "NoiseColor02" (Variables|StarSettings|GetNoiseColor02) :!class /Script/Engine.MaterialInstanceDynamic)
  (Rendering|Material|SetVectorParameterValue _sky_material_4 "NoiseColor03" (Variables|StarSettings|GetNoiseColor03) :!class /Script/Engine.MaterialInstanceDynamic)
  (CallFunction|SetInterpolateParam))

(fn SetInterpolateParam
  (bind _current_time (Variables|TimeDebugSettings|GetCurrent%20Time))
  (bind _timetable (Variables|TimeDebugSettings|GetTimeTable))
  (bind _current_time_2 (Variables|TimeDebugSettings|GetCurrent%20Time))
  (bind _timetable_2 (Variables|TimeDebugSettings|GetTimeTable))
  (bind _directional_light_actor (Variables|Default|GetDirectional%20light%20actor))
  (bind _directional_light_actor_2 (Variables|Default|GetDirectional%20light%20actor))
  (bind _current_time_3 (Variables|TimeDebugSettings|GetCurrent%20Time))
  (bind _timetable_3 (Variables|TimeDebugSettings|GetTimeTable))
  (bind _directional_light_actor_3 (Variables|Default|GetDirectional%20light%20actor))
  (bind _directional_light_actor_4 (Variables|Default|GetDirectional%20light%20actor))
  (bind _current_time_4 (Variables|TimeDebugSettings|GetCurrent%20Time))
  (bind _timetable_4 (Variables|TimeDebugSettings|GetTimeTable))
  (bind _sky_material (Variables|Default|GetSky%20material))
  (bind _x (Math|Vector4|BreakVector4 _timetable))
  (bind (_x_2 _y) (Math|Vector4|BreakVector4 _timetable_2))
  (bind (_x_3 _y_2 _z) (Math|Vector4|BreakVector4 _timetable_3))
  (bind (_x_4 _y_3 _z_2 _w) (Math|Vector4|BreakVector4 _timetable_4))
  (bind _returnvalue (- _current_time 0.0))
  (bind _lightcomponent (Variables|/Script/Engine.Light|GetLightComponent _directional_light_actor))
  (bind _lightcomponent_2 (Variables|/Script/Engine.Light|GetLightComponent _directional_light_actor_3))
  (bind _lightcomponent_3 (Variables|/Script/Engine.Light|GetLightComponent _directional_light_actor_4))
  (bind _lightcomponent_4 (Variables|/Script/Engine.Light|GetLightComponent _directional_light_actor_2))
  (bind _returnvalue_2 (- _y _x_2))
  (bind _returnvalue_3 (- _current_time_2 _x_2))
  (bind _returnvalue_4 (- _z _y_2))
  (bind _returnvalue_5 (- _current_time_3 _y_2))
  (bind _returnvalue_6 (- _w _z_2))
  (bind _returnvalue_7 (- _current_time_4 _z_2))
  (bind _returnvalue_8 (- _x 0.0))
  (bind _returnvalue_9 (/ _returnvalue_3 _returnvalue_2))
  (bind _returnvalue_10 (/ _returnvalue_5 _returnvalue_4))
  (bind _returnvalue_11 (/ _returnvalue_7 _returnvalue_6))
  (bind _returnvalue_12 (/ _returnvalue _returnvalue_8))
  (if (and (> _current_time_2 _x_2) (<= _current_time_2 _y))
    (Variables|TempSettings|SetTempCloudBrightColor (Math|Color|Lerp(LinearColor) (Variables|MorningSettings|GetMorningCloudBrightColor) (Variables|NoonSettings|GetNoonCloudBrightColor) _returnvalue_9))
    (Variables|TempSettings|SetTempCloudDarkColor (Math|Color|Lerp(LinearColor) (Variables|MorningSettings|GetMorningCloudDarkColor) (Variables|NoonSettings|GetNoonCloudDarkColor) _returnvalue_9))
    (Variables|TempSettings|SetTempSkyZenithColor (Math|Color|Lerp(LinearColor) (Variables|MorningSettings|GetMorningSkyZenithColor) (Variables|NoonSettings|GetNoonSkyZenithColor) _returnvalue_9))
    (Variables|TempSettings|SetTempSkyHorizonColor (Math|Color|Lerp(LinearColor) (Variables|MorningSettings|GetMorningSkyHorizonColor) (Variables|NoonSettings|GetNoonSkyHorizonColor) _returnvalue_9))
    (Transformation|SetActorRotation _directional_light_actor_2 (Math|Rotator|MakeRotator 0.0 (Math|Float|Lerp 0.0 -9e+01 _returnvalue_9) 0.0))
    (Rendering|Components|Light|SetLightColor _lightcomponent_4 (Math|Color|Lerp(LinearColor) (Variables|MorningSettings|GetMorningMainLightColor) (Variables|NoonSettings|GetNoonMainLightColor) _returnvalue_9) true)
    (Rendering|Components|Light|SetIntensity _lightcomponent_4 (Math|Float|Lerp (Variables|MorningSettings|GetMorningMainLightIntensity) (Variables|NoonSettings|GetNoonMainLightIntensity) _returnvalue_9))
    (Variables|StarSettings|SetStars%20Brightness (Math|Float|Lerp (Variables|MorningSettings|GetMorning%20Star%20Brightness) (Variables|NoonSettings|GetNoon%20Star%20Brightness) _returnvalue_9))
    (elif (and (> _current_time_3 _y_2) (<= _current_time_3 _z))
      (Variables|TempSettings|SetTempCloudBrightColor (Math|Color|Lerp(LinearColor) (Variables|NoonSettings|GetNoonCloudBrightColor) (Variables|DuskSettings|GetDuskCloudBrightColor) _returnvalue_10))
      (Variables|TempSettings|SetTempCloudDarkColor (Math|Color|Lerp(LinearColor) (Variables|NoonSettings|GetNoonCloudDarkColor) (Variables|DuskSettings|GetDuskCloudDarkColor) _returnvalue_10))
      (Variables|TempSettings|SetTempSkyZenithColor (Math|Color|Lerp(LinearColor) (Variables|NoonSettings|GetNoonSkyZenithColor) (Variables|DuskSettings|GetDuskSkyZenithColor) _returnvalue_10))
      (Variables|TempSettings|SetTempSkyHorizonColor (Math|Color|Lerp(LinearColor) (Variables|NoonSettings|GetNoonSkyHorizonColor) (Variables|DuskSettings|GetDuskSkyHorizonColor) _returnvalue_10))
      (Transformation|SetActorRotation _directional_light_actor_3 (Math|Rotator|MakeRotator 0.0 (Math|Float|Lerp -9e+01 -1.8e+02 _returnvalue_10) 0.0))
      (Rendering|Components|Light|SetLightColor _lightcomponent_2 (Math|Color|Lerp(LinearColor) (Variables|NoonSettings|GetNoonMainLightColor) (Variables|DuskSettings|GetDuskMainLightColor) _returnvalue_10) true)
      (Rendering|Components|Light|SetIntensity _lightcomponent_2 (Math|Float|Lerp (Variables|NoonSettings|GetNoonMainLightIntensity) (Variables|DuskSettings|GetDuskMainLightIntensity) _returnvalue_10))
      (Variables|StarSettings|SetStars%20Brightness (Math|Float|Lerp (Variables|NoonSettings|GetNoon%20Star%20Brightness) (Variables|DuskSettings|GetDusk%20Star%20Brightness) _returnvalue_10))
      (elif (and (> _current_time_4 _z_2) (<= _current_time_4 _w))
        (Variables|TempSettings|SetTempCloudBrightColor (Math|Color|Lerp(LinearColor) (Variables|DuskSettings|GetDuskCloudBrightColor) (Variables|NightSettings|GetNightCloudBrightColor) _returnvalue_11))
        (Variables|TempSettings|SetTempCloudDarkColor (Math|Color|Lerp(LinearColor) (Variables|DuskSettings|GetDuskCloudDarkColor) (Variables|NightSettings|GetNightCloudDarkColor) _returnvalue_11))
        (Variables|TempSettings|SetTempSkyZenithColor (Math|Color|Lerp(LinearColor) (Variables|DuskSettings|GetDuskSkyZenithColor) (Variables|NightSettings|GetNightSkyZenithColor) _returnvalue_11))
        (Variables|TempSettings|SetTempSkyHorizonColor (Math|Color|Lerp(LinearColor) (Variables|DuskSettings|GetDuskSkyHorizonColor) (Variables|NightSettings|GetNightSkyHorizonColor) _returnvalue_11))
        (Transformation|SetActorRotation _directional_light_actor_4 (Math|Rotator|MakeRotator 0.0 (Math|Float|Lerp -1.8e+02 -2.7e+02 _returnvalue_11) 0.0))
        (Rendering|Components|Light|SetLightColor _lightcomponent_3 (Math|Color|Lerp(LinearColor) (Variables|DuskSettings|GetDuskMainLightColor) (Variables|NightSettings|GetNightMainLightColor) _returnvalue_11) true)
        (Rendering|Components|Light|SetIntensity _lightcomponent_3 (Math|Float|Lerp (Variables|DuskSettings|GetDuskMainLightIntensity) (Variables|NightSettings|GetNightMainLightIntensity) _returnvalue_11))
        (Variables|StarSettings|SetStars%20Brightness (Math|Float|Lerp (Variables|DuskSettings|GetDuskMainLightIntensity) (Variables|NightSettings|GetNight%20Star%20Brightness) _returnvalue_11))
        (else
          (Variables|TempSettings|SetTempCloudBrightColor (Math|Color|Lerp(LinearColor) (Variables|NightSettings|GetNightCloudBrightColor) (Variables|MorningSettings|GetMorningCloudBrightColor) _returnvalue_12))
          (Variables|TempSettings|SetTempCloudDarkColor (Math|Color|Lerp(LinearColor) (Variables|NightSettings|GetNightCloudDarkColor) (Variables|MorningSettings|GetMorningCloudDarkColor) _returnvalue_12))
          (Variables|TempSettings|SetTempSkyZenithColor (Math|Color|Lerp(LinearColor) (Variables|NightSettings|GetNightSkyZenithColor) (Variables|MorningSettings|GetMorningSkyZenithColor) _returnvalue_12))
          (Variables|TempSettings|SetTempSkyHorizonColor (Math|Color|Lerp(LinearColor) (Variables|NightSettings|GetNightSkyHorizonColor) (Variables|MorningSettings|GetMorningSkyHorizonColor) _returnvalue_12))
          (Transformation|SetActorRotation _directional_light_actor (Math|Rotator|MakeRotator 0.0 (Math|Float|Lerp -2.7e+02 0.0 _returnvalue_12) 0.0))
          (Rendering|Components|Light|SetLightColor _lightcomponent (Math|Color|Lerp(LinearColor) (Variables|NightSettings|GetNightMainLightColor) (Variables|MorningSettings|GetMorningMainLightColor) _returnvalue_12) true)
          (Rendering|Components|Light|SetIntensity _lightcomponent (Math|Float|Lerp (Variables|NightSettings|GetNightMainLightIntensity) (Variables|MorningSettings|GetMorningMainLightIntensity) _returnvalue_12))
          (Variables|StarSettings|SetStars%20Brightness (Math|Float|Lerp (Variables|NightSettings|GetNight%20Star%20Brightness) (Variables|MorningSettings|GetMorning%20Star%20Brightness) _returnvalue_12))))))
  (Rendering|Material|SetVectorParameterValue _sky_material "CloudBrightColor" (Variables|TempSettings|GetTempCloudBrightColor) :!class /Script/Engine.MaterialInstanceDynamic)
  (Rendering|Material|SetVectorParameterValue _sky_material "CloudDarkColor" (Variables|TempSettings|GetTempCloudDarkColor) :!class /Script/Engine.MaterialInstanceDynamic)
  (Rendering|Material|SetVectorParameterValue _sky_material "Zenith color" (Variables|TempSettings|GetTempSkyZenithColor) :!class /Script/Engine.MaterialInstanceDynamic)
  (Rendering|Material|SetVectorParameterValue _sky_material "Horizon color" (Variables|TempSettings|GetTempSkyHorizonColor) :!class /Script/Engine.MaterialInstanceDynamic)
  (Rendering|Material|SetScalarParameterValue _sky_material "Stars Brightness" (Variables|StarSettings|GetStars%20Brightness) :!class /Script/Engine.MaterialInstanceDynamic)
  (Rendering|Material|SetScalarParameterValue _sky_material "Lunar Inclination" (Variables|MoonSettings|GetMoon%20Inclination) :!class /Script/Engine.MaterialInstanceDynamic)
  (Rendering|Material|SetScalarParameterValue _sky_material "Moon Scale" (Variables|MoonSettings|GetMoon%20Size) :!class /Script/Engine.MaterialInstanceDynamic)
  (Rendering|Material|SetScalarParameterValue _sky_material "Lunar Phase" (Math|Conversions|ToFloat(Integer) (Math|Float|Round (Variables|MoonSettings|GetMoon%20Phase))) :!class /Script/Engine.MaterialInstanceDynamic)
  (Rendering|Material|SetVectorParameterValue _sky_material "Moon Color" (Variables|MoonSettings|GetMoon%20Color) :!class /Script/Engine.MaterialInstanceDynamic)
  (Rendering|Material|SetScalarParameterValue _sky_material "Moon Rotation" (Variables|MoonSettings|GetMoon%20Rotation) :!class /Script/Engine.MaterialInstanceDynamic)
  (Rendering|Material|SetScalarParameterValue _sky_material "UseCustomMoonTexture" (Math|Float|SelectFloat 1.0 0.0 (Variables|MoonSettings|GetUseCustomMoonTexture)) :!class /Script/Engine.MaterialInstanceDynamic)
  (Rendering|Material|SetTextureParameterValue _sky_material "CustomMoonTexture" (Variables|MoonSettings|GetCustomMoonTexture))
  (Rendering|Material|SetScalarParameterValue _sky_material "Moon Intensity" (Variables|MoonSettings|GetMoon%20Intensity) :!class /Script/Engine.MaterialInstanceDynamic)
  (CallFunction|UpdateSunDirection))